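; Player controller that shows the mouse cursor and turns touch drags into panning of the BP_FlyOrthCamera pawn cached at BeginPlay.
; Each touch move scales the distance since the last position along the direction from touch-down, then feeds it with swapped axes into the pawn's FloatingMove.
; LastTouchPos updates on move and release, but not on press.
; Two debug keys add pitch or print, and older movement logic remains unconnected.
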(event EventBeginPlay
  (Variables|Default|SetbShowMouseCursor true)
  (bind _asbp_fly_orth_camera (Utilities|Casting|CastToBP_FlyOrthCamera (Pawn|GetControlledPawn)))
  (Variables|Default|SetCurrCameraPawn _asbp_fly_orth_camera))

(event EventTick
  (params (DeltaSeconds :type Float%20%28single-precision%29)))

(event Input|KeyboardEvents|DebugKey5
  (params (Key :type Key%20Structure :default "None") (ActionValue :type Input%20Action%20Value%20Structure))
  (:Pressed
    (Class|PlayerController|AddPitchInput 5.0)
    (Development|PrintString "+ 5")))

(event Input|KeyboardEvents|DebugKey6
  (params (Key :type Key%20Structure :default "None") (ActionValue :type Input%20Action%20Value%20Structure))
  (:Pressed
    (Development|PrintString (Utilities|GetDisplayName 0))))

(event Input|TouchEvents|InputTouch
  (params (Location :type Vector) (FingerIndex :type ETouchIndex%20Enum))
  (:Pressed
    (Variables|Default|SetTouchDownPos Location))
  (:Released
    (Variables|Default|SetLastTouchPos Location))
  (:Moved
    (Class|PawnMovementComponent|AddInputVector (Variables|/Game/Core/BP_FlyOrthCamera.BP_FlyOrthCamera_C|GetFloatingMove (Variables|Default|GetCurrCameraPawn)) (Math|Vector|MakeVector (.Y (Math|Vector|BreakVector (* (Math|Vector|Distance2D(Vector) (Variables|Default|GetLastTouchPos) Location) (Math|Vector|GetUnitDirection(Vector) (Variables|Default|GetTouchDownPos) Location) 22.0))) (* (.X (Math|Vector|BreakVector (* (Math|Vector|Distance2D(Vector) (Variables|Default|GetLastTouchPos) Location) (Math|Vector|GetUnitDirection(Vector) (Variables|Default|GetTouchDownPos) Location) 22.0))) -1.0) 0.0) false)
    (Variables|Default|SetLastTouchPos Location)))

(fn ConstructionScript)